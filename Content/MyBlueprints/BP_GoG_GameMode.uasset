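; BP_GoG_GameMode is a game mode that handles player login and team-based spawning of BP_IdolCharactter.
; On PostLogin it sorts PlayerStarts by the "Player 1" tag into Command1 and Command2, then notifies the Hero_PC via ClientOnPostLogin.
; SpawnPlayer checks for a valid controlled pawn, calls DestroyActor, then spawns and possesses a new character.
; The first PlayerArray entry uses Command1's first start; others use Command2's.
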(event `self.K2_PostLogin`
  (params (NewPlayer :type "PlayerController Object Reference"))
  (`/Engine/EditorBlueprintResources/ActorMacros.Switch Has Authority`
    (:`Authority`
      _)
    (:`Remote`
      _))
  (set `self.PlayerController` NewPlayer)
  (bind _outactors (`GameplayStatics.GetAllActorsOfClass` "/Script/Engine.PlayerStart"))
  (for _array_element _outactors
    (if (== (`PlayerStart.PlayerStartTag` _array_element) "Player 1")
      (`KismetArrayLibrary.Array_AddUnique` (`self.Command 1`))
      (else
        (`KismetArrayLibrary.Array_AddUnique` (`self.Command 2`)))))
  (bind _ashero_pc (cast `/Game/MyBlueprints/Hero_PC` (`self.PlayerController`)))
  (`/Game/MyBlueprints/Hero_PC.ClientOnPostLogin` _ashero_pc))

(event `SpawnPlayer`
  (params (PlayerController :type "PlayerController Object Reference"))
  (bind _output_get (set `self.PlayerController` PlayerController))
  (`/Engine/EditorBlueprintResources/StandardMacros.IsValid` (`Controller.K2_GetPawn` _output_get)
    (:`Is Valid`
      (`self.K2_DestroyActor`)
      (if (== (`PlayerState.PlayerId` (`Controller.PlayerState` (`self.PlayerController`))) (`PlayerState.PlayerId` (`|GetArrayItem` (`GameStateBase.PlayerArray` (`GameplayStatics.GetGameState`)))))
        (bind _returnvalue (`|SpawnActorFromClass` "/Game/MyBlueprints/Characters/BP_IdolCharactter.BP_IdolCharactter_C" (`self.GetTransform` (`|GetArrayItem` (`self.Command 1`))) "Undefined" "OverrideRootScale" null null))
        (`Controller.Possess` (`self.PlayerController`) _returnvalue)
        (else
          (bind _returnvalue_2 (`|SpawnActorFromClass` "/Game/MyBlueprints/Characters/BP_IdolCharactter.BP_IdolCharactter_C" (`self.GetTransform` (`|GetArrayItem` (`self.Command 2`))) "Undefined" "OverrideRootScale" null null))
          (`Controller.Possess` (`self.PlayerController`) _returnvalue_2))))))

(fn `UserConstructionScript`)