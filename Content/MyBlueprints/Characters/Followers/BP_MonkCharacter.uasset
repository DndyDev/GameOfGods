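; Monk character Blueprint, filed with the followers, that provides a HealAlly function for restoring ally health.
; HealAlly casts the target to BP_FollowerCharacter and adds a fixed amount to its Health.
; If that target also casts to BP_IdolCharactter and the monk's controller is Hero_PC, it deducts a coin and adds health again.
; The event graph holds only disabled or empty events, and nothing here calls HealAlly.
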(event `Key|One`
  (params (Key :type "Key Structure")))

(event `OnActorEndOverlap_Event_0`
  (params (OverlappedActor :type "Actor Object Reference") (OtherActor :type "Actor Object Reference")))

(fn `healAlly`
  (params (Character :type "Character Object Reference"))
  (bind _asbp_follower_character (cast `/Game/MyBlueprints/Characters/BP_FollowerCharacter` Character))
  (set `/Game/MyBlueprints/Characters/BP_PlayerCharacter.Health` (+ (`/Game/MyBlueprints/Characters/BP_PlayerCharacter.Health` _asbp_follower_character) 10) _asbp_follower_character)
  (bind _asbp_idol_charactter (cast `/Game/MyBlueprints/Characters/BP_IdolCharactter` Character))
  (bind _ashero_pc (cast `/Game/MyBlueprints/Hero_PC` (`self.GetController`)))
  (set `/Game/MyBlueprints/Hero_PC.CoinCounter` (- (`/Game/MyBlueprints/Hero_PC.CoinCounter` _ashero_pc) 1) _ashero_pc)
  (set `/Game/MyBlueprints/Characters/BP_PlayerCharacter.Health` (+ (`/Game/MyBlueprints/Characters/BP_PlayerCharacter.Health` _asbp_idol_charactter) 10) _asbp_idol_charactter))

(fn `UserConstructionScript`
  (`parent.UserConstructionScript`))