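; BP_IdolCharactter is a character Blueprint for an Idol that attacks by throwing rocks.
; BeginPlay runs parent setup, then sets Health and pushes it to the HUD counter.
; Each Tick in the Attack task state calls RockThrow, which spawns a scaled Rock at the CastArrow transform, moving along its forward vector, with no cooldown in this graph.
; The Earth function is an empty stub.
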(event `self.ReceiveBeginPlay`
  (`parent.ReceiveBeginPlay`)
  ;[1 1 1] Set Health
  (bind _output_get (set `self.Health` 200))
  (`/Game/MyBlueprints/Widgets/BP_HUDWidget.UpdateHealthCounter` (`self.HUD`) _output_get))

(event `Key|One`
  (params (Key :type "Key Structure")))

(event `self.ReceiveTick`
  (params (DeltaSeconds :type "Float (single-precision)"))
  (`parent.ReceiveTick` DeltaSeconds)
  (switch `/Game/MyBlueprints/Characters/E_PlayerStates` "NewEnumerator0"
    (:`NewEnumerator2`
      (`self.RockThrow`))))

(fn `Earth`)

(fn `RockThrow`
  (bind (_returnvalue_location _returnvalue_rotation) (`KismetMathLibrary.BreakTransform` (`SceneComponent.K2_GetComponentToWorld` (`self.CastArrow`))))
  (`|SpawnActorFromClass` "/Game/MyBlueprints/Rock.Rock_C" (`KismetMathLibrary.MakeTransform` _returnvalue_location _returnvalue_rotation (`self.RockScale`)) "Undefined" "OverrideRootScale" null (`SceneComponent.GetForwardVector` (`self.CastArrow`)) null))

(fn `UserConstructionScript`
  (`parent.UserConstructionScript`))