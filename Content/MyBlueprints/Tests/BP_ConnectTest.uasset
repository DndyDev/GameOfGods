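; Functional test that checks whether every expected player has connected to the lobby.
; On StartTest it casts the game mode to LobbyGM and compares the AllPlayerControllers count with MaxPlayer in a single immediate check.
; A match finishes as Succeeded, while a mismatch finishes with the Default result, not Failed, and a net error message giving both counts.
; A failed cast never calls FinishTest.
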(event `self.ReceiveStartTest`
  (bind _aslobby_gm (cast `/Game/MyBlueprints/Lobby/LobbyGM` (`GameplayStatics.GetGameMode`)))
  (bind _returnvalue (`KismetArrayLibrary.Array_Length` (`/Game/MyBlueprints/Lobby/LobbyGM.AllPlayerControllers` _aslobby_gm)))
  (bind _maxplayer (`/Game/MyBlueprints/Lobby/LobbyGM.MaxPlayer` _aslobby_gm))
  (if (== _returnvalue _maxplayer)
    (`self.FinishTest` "Succeeded")
    (else
      (`self.FinishTest` "Default" (`KismetTextLibrary.Conv_TextToString` (`|FormatText` "Net error {Conttrollers} of {MaxPlayers } connected" _returnvalue _maxplayer))))))

(fn `UserConstructionScript`)