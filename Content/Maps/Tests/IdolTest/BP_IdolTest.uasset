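; BP_IdolTest is a functional test that checks whether the Idol character's rock throw damages a follower.
; On test start it calls RockThrow on the testing character, then waits briefly for the rock to land.
; It then passes if the target follower's Health is below MaxHealth, and otherwise fails with a no-damage message.
; A failed cast on either character stops the graph without finishing the test.
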(event `self.ReceiveStartTest`
  (bind _asbp_idol_charactter (cast `/Game/MyBlueprints/Characters/BP_IdolCharactter` (`self.TestingCharacter`)))
  (`/Game/MyBlueprints/Characters/BP_IdolCharactter.RockThrow` _asbp_idol_charactter)
  (`KismetSystemLibrary.Delay` 2.0)
  (bind _asbp_follower_character (cast `/Game/MyBlueprints/Characters/BP_FollowerCharacter` (`self.Target`)))
  (if (< (`/Game/MyBlueprints/Characters/BP_PlayerCharacter.Health` _asbp_follower_character) (`/Game/MyBlueprints/Characters/BP_PlayerCharacter.MaxHealth` _asbp_follower_character))
    (`self.FinishTest` "Succeeded")
    (else
      (`self.FinishTest` "Failed" "Rock not apply damage"))))

(fn `UserConstructionScript`)